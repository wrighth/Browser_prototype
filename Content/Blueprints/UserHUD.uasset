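; HUD for a genome viewer that draws a crosshair and shows details of hit gene models and track features.
; Each DrawHUD scans Exon_Intron_Model actors for hit flags, scanning Track_BP actors within the loop for every unhit model.
; Hits print gene info, plus feature data for tracks, as colored text over offset black shadows, then clear their flag.
; BeginPlay adds the FileNameInput widget to the viewport.
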(event EventBeginPlay
  (bind _returnvalue (UserInterface|CreateWidget "/Game/Blueprints/FileNameInput.FileNameInput_C" 0 "0.000000,0.000000,0.000000|0.000000,0.000000,0.000000|1.000000,1.000000,1.000000"))
  (UserInterface|Viewport|AddtoViewport _returnvalue 0))

(event EventTick
  (params (DeltaSeconds :type Float%20%28single-precision%29)))

(event EventDrawHUD
  (params (SizeX :type Integer) (SizeY :type Integer))
  (Canvas|DrawTexture "/Game/Crosshair.Crosshair" (Math|Conversions|ToFloat(Integer) (/ SizeX 2)) (Math|Conversions|ToFloat(Integer) (/ SizeY 2)) 6.0 6.0 0.0 0.0 0.0 0.0 "(R=1.000000,G=1.000000,B=1.000000,A=1.000000)")
  (bind _outactors (Actor|GetAllActorsOfClass "/Game/Blueprints/Exon_Intron_Model.Exon_Intron_Model_C"))
  (for _array_element _outactors
    (if (Variables|/Game/Blueprints/Exon_Intron_Model.Exon_Intron_Model_C|GetIsHitExonIntron _array_element)
      (HUD|DrawText (Utilities|String|Append "End position: " (Utilities|Array|Get(acopy) (Variables|/Game/Blueprints/Exon_Intron_Model.Exon_Intron_Model_C|GetInfoArray _array_element))) "(R=0.000000,G=0.000000,B=0.000000,A=1.000000)" 9.0 69.0 0 1.25 false)
      (HUD|DrawText (Utilities|String|Append "Start position: " (Utilities|Array|Get(acopy) (Variables|/Game/Blueprints/Exon_Intron_Model.Exon_Intron_Model_C|GetInfoArray _array_element) 1)) "(R=0.000000,G=0.000000,B=0.000000,A=1.000000)" 9.0 49.0 0 1.25 false)
      (HUD|DrawText (Utilities|String|Append "On chromosome: " (Utilities|Array|Get(acopy) (Variables|/Game/Blueprints/Exon_Intron_Model.Exon_Intron_Model_C|GetInfoArray _array_element) 2)) "(R=0.000000,G=0.000000,B=0.000000,A=1.000000)" 9.0 29.0 0 1.25 false)
      (HUD|DrawText (Utilities|String|Append "Gene name: " (Utilities|Array|Get(acopy) (Variables|/Game/Blueprints/Exon_Intron_Model.Exon_Intron_Model_C|GetInfoArray _array_element) 3)) "(R=0.000000,G=0.000000,B=0.000000,A=1.000000)" 9.0 9.0 0 1.25 false)
      (HUD|DrawText (Utilities|String|Append "End position: " (Utilities|Array|Get(acopy) (Variables|/Game/Blueprints/Exon_Intron_Model.Exon_Intron_Model_C|GetInfoArray _array_element))) "(R=0.000000,G=0.658824,B=1.000000,A=1.000000)" 8.0 68.0 0 1.25 false)
      (HUD|DrawText (Utilities|String|Append "Start position: " (Utilities|Array|Get(acopy) (Variables|/Game/Blueprints/Exon_Intron_Model.Exon_Intron_Model_C|GetInfoArray _array_element) 1)) "(R=0.000000,G=0.658824,B=1.000000,A=1.000000)" 8.0 48.0 0 1.25 false)
      (HUD|DrawText (Utilities|String|Append "On chromosome: " (Utilities|Array|Get(acopy) (Variables|/Game/Blueprints/Exon_Intron_Model.Exon_Intron_Model_C|GetInfoArray _array_element) 2)) "(R=0.000000,G=0.658824,B=1.000000,A=1.000000)" 8.0 28.0 0 1.25 false)
      (HUD|DrawText (Utilities|String|Append "Gene name: " (Utilities|Array|Get(acopy) (Variables|/Game/Blueprints/Exon_Intron_Model.Exon_Intron_Model_C|GetInfoArray _array_element) 3)) "(R=0.000000,G=0.658824,B=1.000000,A=1.000000)" 8.0 8.0 0 1.25 false)
      (Variables|/Game/Blueprints/Exon_Intron_Model.Exon_Intron_Model_C|SetIsHitExonIntron _array_element false)
      (else
        (bind _outactors_2 (Actor|GetAllActorsOfClass "/Game/Blueprints/Track_BP.Track_BP_C"))
        (for _array_element_2 _outactors_2
          (if (Variables|/Game/Blueprints/Track_BP.Track_BP_C|GetIsHitFeature _array_element_2)
            (HUD|DrawText (Utilities|Array|Get(acopy) (Variables|/Game/Blueprints/Track_BP.Track_BP_C|GetInfoArray _array_element_2) 4) "(R=0,G=0,B=0,A=1)" 9.0 99.0 0 1.25 false)
            (HUD|DrawText (Utilities|String|Append "Start: " (Utilities|Array|Get(acopy) (Variables|/Game/Blueprints/Track_BP.Track_BP_C|GetInfoArray _array_element_2) 1)) "(R=0.000000,G=0.000000,B=0.000000,A=1.000000)" 9.0 119.0 0 1.25 false)
            (HUD|DrawText (Utilities|String|Append "End: " (Utilities|Array|Get(acopy) (Variables|/Game/Blueprints/Track_BP.Track_BP_C|GetInfoArray _array_element_2) 2)) "(R=0.000000,G=0.000000,B=0.000000,A=1.000000)" 9.0 139.0 0 1.25 false)
            (HUD|DrawText (Utilities|String|Append "Height: " (Utilities|Array|Get(acopy) (Variables|/Game/Blueprints/Track_BP.Track_BP_C|GetInfoArray _array_element_2) 3)) "(R=0.000000,G=0.000000,B=0.000000,A=1.000000)" 9.0 159.0 0 1.25 false)
            (HUD|DrawText (Utilities|String|Append "End position: " (Utilities|Array|Get(acopy) (Variables|/Game/Blueprints/Exon_Intron_Model.Exon_Intron_Model_C|GetInfoArray (Variables|/Game/Blueprints/Track_BP.Track_BP_C|GetModelReference _array_element_2)))) "(R=0.000000,G=0.000000,B=0.000000,A=1.000000)" 9.0 69.0 0 1.25 false)
            (HUD|DrawText (Utilities|String|Append "Start position: " (Utilities|Array|Get(acopy) (Variables|/Game/Blueprints/Exon_Intron_Model.Exon_Intron_Model_C|GetInfoArray (Variables|/Game/Blueprints/Track_BP.Track_BP_C|GetModelReference _array_element_2)) 1)) "(R=0.000000,G=0.000000,B=0.000000,A=1.000000)" 9.0 49.0 0 1.25 false)
            (HUD|DrawText (Utilities|String|Append "On chromosome: " (Utilities|Array|Get(acopy) (Variables|/Game/Blueprints/Exon_Intron_Model.Exon_Intron_Model_C|GetInfoArray (Variables|/Game/Blueprints/Track_BP.Track_BP_C|GetModelReference _array_element_2)) 2)) "(R=0.000000,G=0.000000,B=0.000000,A=1.000000)" 9.0 29.0 0 1.25 false)
            (HUD|DrawText (Utilities|String|Append "Gene name: " (Utilities|Array|Get(acopy) (Variables|/Game/Blueprints/Exon_Intron_Model.Exon_Intron_Model_C|GetInfoArray (Variables|/Game/Blueprints/Track_BP.Track_BP_C|GetModelReference _array_element_2)) 3)) "(R=0.000000,G=0.000000,B=0.000000,A=1.000000)" 9.0 9.0 0 1.25 false)
            (HUD|DrawText (Utilities|Array|Get(acopy) (Variables|/Game/Blueprints/Track_BP.Track_BP_C|GetInfoArray _array_element_2) 4) "(R=1.000000,G=0.662745,B=0.000000,A=1.000000)" 8.0 98.0 0 1.25 false)
            (HUD|DrawText (Utilities|String|Append "Start: " (Utilities|Array|Get(acopy) (Variables|/Game/Blueprints/Track_BP.Track_BP_C|GetInfoArray _array_element_2) 1)) "(R=1.000000,G=0.662745,B=0.000000,A=1.000000)" 8.0 118.0 0 1.25 false)
            (HUD|DrawText (Utilities|String|Append "End: " (Utilities|Array|Get(acopy) (Variables|/Game/Blueprints/Track_BP.Track_BP_C|GetInfoArray _array_element_2) 2)) "(R=1.000000,G=0.662745,B=0.000000,A=1.000000)" 8.0 138.0 0 1.25 false)
            (HUD|DrawText (Utilities|String|Append "Height: " (Utilities|Array|Get(acopy) (Variables|/Game/Blueprints/Track_BP.Track_BP_C|GetInfoArray _array_element_2) 3)) "(R=1.000000,G=0.662745,B=0.000000,A=1.000000)" 8.0 158.0 0 1.25 false)
            (HUD|DrawText (Utilities|String|Append "End position: " (Utilities|Array|Get(acopy) (Variables|/Game/Blueprints/Exon_Intron_Model.Exon_Intron_Model_C|GetInfoArray (Variables|/Game/Blueprints/Track_BP.Track_BP_C|GetModelReference _array_element_2)))) "(R=0.000000,G=0.658824,B=1.000000,A=1.000000)" 8.0 68.0 0 1.25 false)
            (HUD|DrawText (Utilities|String|Append "Start position: " (Utilities|Array|Get(acopy) (Variables|/Game/Blueprints/Exon_Intron_Model.Exon_Intron_Model_C|GetInfoArray (Variables|/Game/Blueprints/Track_BP.Track_BP_C|GetModelReference _array_element_2)) 1)) "(R=0.000000,G=0.658824,B=1.000000,A=1.000000)" 8.0 48.0 0 1.25 false)
            (HUD|DrawText (Utilities|String|Append "On chromosome: " (Utilities|Array|Get(acopy) (Variables|/Game/Blueprints/Exon_Intron_Model.Exon_Intron_Model_C|GetInfoArray (Variables|/Game/Blueprints/Track_BP.Track_BP_C|GetModelReference _array_element_2)) 2)) "(R=0.000000,G=0.658824,B=1.000000,A=1.000000)" 8.0 28.0 0 1.25 false)
            (HUD|DrawText (Utilities|String|Append "Gene name: " (Utilities|Array|Get(acopy) (Variables|/Game/Blueprints/Exon_Intron_Model.Exon_Intron_Model_C|GetInfoArray (Variables|/Game/Blueprints/Track_BP.Track_BP_C|GetModelReference _array_element_2)) 3)) "(R=0.000000,G=0.658824,B=1.000000,A=1.000000)" 8.0 8.0 0 1.25 false)
            (Variables|/Game/Blueprints/Track_BP.Track_BP_C|SetIsHitFeature _array_element_2 false)))))))

(fn ConstructionScript)