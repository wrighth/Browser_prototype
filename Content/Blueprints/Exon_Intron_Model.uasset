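; Draggable actor modeling a gene's exon-intron structure as a chain of cylinders.
; The construction script scales and offsets alternating thick and thin segments from ScaleFactors and reads gene identity from InfoArray.
; Clicking opens a gate that follows the deprojected cursor at grab distance; MoveActor lerps it by timeline.
; Both movements re-pin every Network_Model spline mesh to matching genes, while a camera trace each tick flags whether this actor is hit.
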(event Custom|Tick%201
  (bind _returnvalue (Game|GetPlayerCameraManager 0))
  (bind _returnvalue_2 (Transformation|GetActorLocation _returnvalue))
  (bind (_outhit _returnvalue_3) (Collision|LineTraceByChannel _returnvalue_2 (+ _returnvalue_2 (* (Transformation|GetActorForwardVector _returnvalue) 7.5e+03)) "TraceTypeQuery1" false 0 "None" false))
  (if _returnvalue_3
    (if (== (.HitActor (Collision|BreakHitResult _outhit)) self)
      (Variables|Default|SetIsHitExonIntron true)
      (else
        (Variables|Default|SetIsHitExonIntron false)))
    (else
      (Variables|Default|SetIsHitExonIntron false))))

(event Custom|Tick%202
  (bind _returnvalue (Game|GetPlayerController 0))
  (bind (_worldlocation _worlddirection) (Game|Player|ConvertMouseLocationToWorldSpace _returnvalue))
  (Utilities|FlowControl|Gate true
    (:Exit
      (bind _output_get (Variables|Default|SetTrueLocation (+ _worldlocation (* _worlddirection (Variables|Default|GetDirectionMultiplier)))))
      (Transformation|SetActorLocation _output_get false false)
      (bind _foundwidgets (Widget|GetAllWidgetsOfClass "/Game/Blueprints/UserUI.UserUI_C" true))
      (Input|SetInputModeGameandUI (Game|GetPlayerController 0) (Utilities|Array|Get(acopy) _foundwidgets) false true)
      (bind _outactors (Actor|GetAllActorsOfClass "Exon_Intron_Model_C"))
      (for _array_element _outactors
        (bind _outactors_2 (Actor|GetAllActorsOfClass "/Game/Blueprints/Network_Model.Network_Model_C"))
        (for _array_element_2 _outactors_2
          (if (Utilities|Enum|Equal(Enum) (Variables|/Game/Blueprints/Network_Model.Network_Model_C|GetStart%20Gene _array_element_2) (Variables|Exon_Intron_Model_C|GetGeneName _array_element))
            (for _array_element_3 (Actor|GetComponentsByClass _array_element_2 "/Script/Engine.SplineMeshComponent")
              (SplineMesh|SetStartPosition _array_element_3 (Transformation|GetActorLocation _array_element) true))
            (elif (Utilities|Enum|Equal(Enum) (Variables|/Game/Blueprints/Network_Model.Network_Model_C|GetEnd%20Gene _array_element_2) (Variables|Exon_Intron_Model_C|GetGeneName _array_element))
              (for _array_element_4 (Actor|GetComponentsByClass _array_element_2 "/Script/Engine.SplineMeshComponent")
                (SplineMesh|SetEndPosition _array_element_4 (Transformation|GetActorLocation _array_element) true)))))))))

(event Custom|MoveActor
  (params (StartLocation :type Vector) (EndLocation :type Vector))
  (bind _floattrack (Timeline|Move_Timeline PlayFromStart)
    (:Update
      (Transformation|SetActorLocation (Math|Vector|Lerp(Vector) StartLocation EndLocation _floattrack) false false)
      (bind _outactors (Actor|GetAllActorsOfClass "Exon_Intron_Model_C"))
      (for _array_element _outactors
        (bind _outactors_2 (Actor|GetAllActorsOfClass "/Game/Blueprints/Network_Model.Network_Model_C"))
        (for _array_element_2 _outactors_2
          (if (Utilities|Enum|Equal(Enum) (Variables|/Game/Blueprints/Network_Model.Network_Model_C|GetStart%20Gene _array_element_2) (Variables|Exon_Intron_Model_C|GetGeneName _array_element))
            (for _array_element_3 (Actor|GetComponentsByClass _array_element_2 "/Script/Engine.SplineMeshComponent")
              (SplineMesh|SetStartPosition _array_element_3 (Transformation|GetActorLocation _array_element) true))
            (elif (Utilities|Enum|Equal(Enum) (Variables|/Game/Blueprints/Network_Model.Network_Model_C|GetEnd%20Gene _array_element_2) (Variables|Exon_Intron_Model_C|GetGeneName _array_element))
              (for _array_element_4 (Actor|GetComponentsByClass _array_element_2 "/Script/Engine.SplineMeshComponent")
                (SplineMesh|SetEndPosition _array_element_4 (Transformation|GetActorLocation _array_element) true)))))))
    (:Finished
      (Variables|Default|SetTrueLocation EndLocation))))

(event EventTick
  (params (DeltaSeconds :type Float%20%28single-precision%29))
  (CallFunction|Tick1)
  (CallFunction|Tick2))

(event MouseInput|EventActorOnClicked
  (params (ButtonPressed :type Key%20Structure :default "AnyKey"))
  (bind _returnvalue (Game|GetPlayerController 0))
  (bind (_worldlocation _worlddirection) (Game|Player|ConvertMouseLocationToWorldSpace _returnvalue))
  (Variables|/Script/Engine.PlayerController|SetCurrentMouseCursor (Game|GetPlayerController 0) "GrabHandClosed")
  (Variables|Default|SetDirectionMultiplier (Math|Vector|VectorLength (- (Transformation|GetActorLocation) (Transformation|GetActorLocation (Game|Player|GetPlayerPawn 0)))))
  (bind _foundwidgets (Widget|GetAllWidgetsOfClass "/Game/Blueprints/UserUI.UserUI_C" true))
  (Input|SetInputModeUIOnly (Game|GetPlayerController 0) (Utilities|Array|Get(acopy) _foundwidgets) false)
  (Utilities|FlowControl|Gate true) ; enters at Open
)

(event EventActorOnReleased
  (params (ButtonReleased :type Key%20Structure :default "AnyKey"))
  (bind _returnvalue (Game|GetPlayerController 0))
  (bind (_worldlocation _worlddirection) (Game|Player|ConvertMouseLocationToWorldSpace _returnvalue))
  (Variables|/Script/Engine.PlayerController|SetCurrentMouseCursor (Game|GetPlayerController 0) "GrabHand")
  (Utilities|FlowControl|Gate true) ; enters at Close
)

(event MouseInput|EventActorBeginCursorOver
  (Variables|/Script/Engine.PlayerController|SetCurrentMouseCursor (Game|GetPlayerController 0) "GrabHand"))

(event MouseInput|EventActorEndCursorOver
  (Variables|/Script/Engine.PlayerController|SetCurrentMouseCursor (Game|GetPlayerController 0) "Default"))

(fn ConstructionScript
  (bind _scalefactors (Variables|Default|GetScaleFactors))
  (bind _infoarray (Variables|Default|GetInfoArray))
  (bind _item (Utilities|Array|Get(acopy) _scalefactors))
  (bind _returnvalue (* 5e+01 _item))
  (Variables|Default|SetTrueLocation (.Location (Math|Transform|BreakTransform (Variables|Default|GetModelTransform))))
  (LocalVariables|Setiter 1)
  (bind _output_get (LocalVariables|SetExon_Num (Variables|Default|GetSegments)))
  (bind _returnvalue_2 (AddComponent|AddStaticMeshComponent false (Math|Transform|MakeTransform "0, 0, 0" "90.000000, 0, 0" (Math|Vector|MakeVector 1.0 1.0 (Utilities|Array|Get(acopy) (Variables|Default|GetScaleFactors))))))
  (Components|StaticMesh|SetStaticMesh _returnvalue_2 "/Engine/BasicShapes/Cylinder.Cylinder")
  (bind _returnvalue_3 (Class|GenerateGeneObjects|GenerateOffset _returnvalue (Utilities|Array|Get(acopy) _scalefactors) (Utilities|Array|Get(acopy) _scalefactors) (Utilities|Array|Get(acopy) _scalefactors 1)))
  (bind _output_get_2 (LocalVariables|Setcurrent_offset _returnvalue_3))
  (Utilities|Array|Add (Variables|Default|Getoffsets) _output_get_2)
  (while (< (stale _output_get_3) _output_get)
    (if (LocalVariables|GetisIntron)
      (LocalVariables|Setxy_scale 0.5)
      (else
        (LocalVariables|Setxy_scale 1.0)))
    (bind _returnvalue_4 (AddComponent|AddStaticMeshComponent false (Math|Transform|MakeTransform (Math|Vector|MakeVector (+ 0.0 (LocalVariables|Getcurrent_offset)) 0.0 0.0) "90.000000, 0, 0" (Math|Vector|MakeVector (LocalVariables|Getxy_scale) (LocalVariables|Getxy_scale) (Utilities|Array|Get(acopy) _scalefactors (LocalVariables|Getiter))))))
    (Components|StaticMesh|SetStaticMesh _returnvalue_4 "/Engine/BasicShapes/Cylinder.Cylinder")
    (if (LocalVariables|GetisIntron)
      (LocalVariables|SetisIntron false)
      (else
        (LocalVariables|SetisIntron true)))
    (bind _output_get_3 (LocalVariables|Setiter (+ (LocalVariables|Getiter) 1)))
    (if (< _output_get_3 (LocalVariables|GetExon_Num))
      (bind _returnvalue_5 (Class|GenerateGeneObjects|GenerateOffset _returnvalue (Utilities|Array|Get(acopy) _scalefactors) (Utilities|Array|Get(acopy) _scalefactors (- (LocalVariables|Getiter) 1)) (Utilities|Array|Get(acopy) _scalefactors (LocalVariables|Getiter))))
      (bind _output_get_4 (LocalVariables|Setcurrent_offset (+ _returnvalue_5 (LocalVariables|Getcurrent_offset))))
      (Variables|Default|SetLastOffset _output_get_4)
      (Utilities|Array|Add (Variables|Default|Getoffsets) _output_get_4)))
  (Transformation|SetActorTransform (Math|Transform|MakeTransform (Variables|Default|GetTrueLocation)))
  (Variables|Default|SetChrName (Utilities|Array|Get(acopy) _infoarray 2))
  (Variables|Default|SetGeneName (Utilities|Array|Get(acopy) _infoarray 3)))