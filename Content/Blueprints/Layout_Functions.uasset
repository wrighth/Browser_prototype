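; Layout helper Blueprint that decides whether genes need automatic placement and generates fallback positions for them.
; NeedsAutoLayout reads positions from a file array via GetGenePositions and returns true only when every one is effectively the zero vector.
; GeneratePositions builds one vector per gene, stacking them along Z at a fixed spacing by array index.
; The event graph and construction script are empty.
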(event EventBeginPlay)

(event Collision|EventActorBeginOverlap
  (params (OtherActor :type Actor%20Object%20Reference)))

(event EventTick
  (params (DeltaSeconds :type Float%20%28single-precision%29)))

(fn ConstructionScript)

(fn NeedsAutoLayout
  (params (FileArray :type Array%20of%20Strings))
  (bind _returnvalue (Class|ReadInputFile|GetGenePositions FileArray))
  (for _array_element _returnvalue
    (if (Math|Vector|NotEqual(Vector) _array_element "0, 0, 0" 0.0001)
      (Math|Integer|IncrementInt (LocalVariables|Getiter))))
  (if (== (LocalVariables|Getiter) 0)
    (return true)
    (else
      (return false))))

(fn GeneratePositions
  (params (Genes :type Array%20of%20Strings))
  (for (_ _array_index) Genes
    (Utilities|Array|Add (LocalVariables|GetReturnVectors) (Math|Vector|MakeVector 0.0 0.0 (Math|Conversions|ToFloat(Integer) (* _array_index 400)))))
  (return (LocalVariables|GetReturnVectors)))