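; Track_BP is an actor that draws one genomic track feature as a colored bar on a referenced gene model.
; The construction script maps feature start and end against the gene's coordinates and model length to place, stretch and rotate a cube, with feature height setting its Z scale.
; It tints the cube through a dynamic material and fills an info array.
; Each tick, a camera-forward line trace sets whether the player is looking at it.
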(event EventBeginPlay)

(event EventTick
  (params (DeltaSeconds :type Float%20%28single-precision%29))
  (bind _returnvalue (Game|GetPlayerCameraManager 0))
  (bind _returnvalue_2 (Transformation|GetActorLocation _returnvalue))
  (bind (_outhit _returnvalue_3) (Collision|LineTraceByChannel _returnvalue_2 (+ _returnvalue_2 (* (Transformation|GetActorForwardVector _returnvalue) 7.5e+03)) "TraceTypeQuery1" false 0 "None" false))
  (if _returnvalue_3
    (if (== (.HitActor (Collision|BreakHitResult _outhit)) self)
      (Variables|Default|SetIsHitFeature true)
      (else
        (Variables|Default|SetIsHitFeature false)))
    (else
      (Variables|Default|SetIsHitFeature false))))

(fn ConstructionScript
  (bind _modelreference (Variables|Default|GetModelReference))
  (bind _modelreference_2 (Variables|Default|GetModelReference))
  (bind _scalefactors (Variables|/Game/Blueprints/Exon_Intron_Model.Exon_Intron_Model_C|GetScaleFactors _modelreference_2))
  (bind _modeltransform (Variables|/Game/Blueprints/Exon_Intron_Model.Exon_Intron_Model_C|GetModelTransform _modelreference))
  (bind _returnvalue (Utilities|Array|Length _scalefactors))
  (bind _location (Math|Transform|BreakTransform _modeltransform))
  (bind (_x _y _z) (Math|Vector|BreakVector _location))
  (bind _returnvalue_2 (Class|GenerateGeneObjects|GenerateOffset 5e+01 (Utilities|Array|Get(acopy) _scalefactors) (Utilities|Array|Get(acopy) _scalefactors (- _returnvalue 1)) (Utilities|Array|Get(acopy) _scalefactors _returnvalue)))
  (Variables|Default|SetAbsoluteGeneLength (+ _returnvalue_2 (Variables|/Game/Blueprints/Exon_Intron_Model.Exon_Intron_Model_C|GetLastOffset (Variables|Default|GetModelReference))))
  (bind _output_get (Variables|Default|SetGeneStart (Math|Conversions|ToInteger(Byte) (Utilities|Array|Get(acopy) (Variables|/Game/Blueprints/Exon_Intron_Model.Exon_Intron_Model_C|GetInfoArray (Variables|Default|GetModelReference)) 1))))
  (bind _output_get_2 (Variables|Default|SetGeneEnd (Math|Conversions|ToInteger(Byte) (Utilities|Array|Get(acopy) (Variables|/Game/Blueprints/Exon_Intron_Model.Exon_Intron_Model_C|GetInfoArray (Variables|Default|GetModelReference))))))
  (bind _returnvalue_3 (Class|ChipSeqTrack|GenerateFeatureScaleLength _output_get _output_get_2 (Variables|Default|GetFeatureStart) (Variables|Default|GetFeatureEnd)))
  (Variables|Default|SetLengthRatio _returnvalue_3)
  (bind _returnvalue_4 (Class|ChipSeqTrack|GenerateXDisplacement (Variables|Default|GetGeneStart) (Variables|Default|GetGeneEnd) (Variables|Default|GetAbsoluteGeneLength) (Variables|Default|GetFeatureStart) (Variables|Default|GetFeatureEnd)))
  (bind _returnvalue_5 (AddComponent|AddStaticMeshComponent false (Math|Transform|MakeTransform (Math|Vector|MakeVector _returnvalue_4 _y _z) (Math|Rotator|MakeRotator (Variables|Default|GetRotation) 0.0 0.0) (Math|Vector|MakeVector (/ (* (Variables|Default|GetLengthRatio) (Variables|Default|GetAbsoluteGeneLength)) 1e+02) 0.025 (+ (Variables|Default|GetFeatureHeight) 0.4)))))
  (Components|StaticMesh|SetStaticMesh _returnvalue_5 "/Game/StarterContent/Shapes/Shape_Cube.Shape_Cube")
  (bind _returnvalue_6 (Rendering|Material|CreateDynamicMaterialInstance _returnvalue_5 0 "/Game/StarterContent/Materials/M_Basic_Wall.M_Basic_Wall" :!class /Script/Engine.PrimitiveComponent))
  (Rendering|Material|SetVectorParameterValue _returnvalue_6 "Color" (Variables|Default|GetTrackColor) :!class /Script/Engine.MaterialInstanceDynamic)
  (Variables|Default|SetInfoArray (Utilities|Array|MakeArray (Variables|Default|GetTargetChrName) (Utilities|String|ToString(Integer) (Variables|Default|GetFeatureStart)) (Utilities|String|ToString(Integer) (Variables|Default|GetFeatureEnd)) (Utilities|String|ToString(Float) (Variables|Default|GetFeatureHeight)) (Variables|Default|GetTrackName))))