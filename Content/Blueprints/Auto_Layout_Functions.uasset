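; Auto-layout functions that position Exon_Intron_Model gene actors in a gene network visualization.
; NeedsAutoLayout flags files whose gene positions are all zero, and GeneratePositions creates vectors from the gene count.
; Two sort functions rearrange placed genes alphabetically or by connectivity, tallied from each Network_Model's start and end genes.
; Both map gene names to computed locations, apply a fixed rotation and call MoveSpline on each gene.
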(fn NeedsAutoLayout
  (params (FileArray :type Array%20of%20Strings))
  (bind _returnvalue (Class|ReadInputFile|GetGenePositions FileArray))
  (for _array_element _returnvalue
    (if (Math|Vector|NotEqual(Vector) _array_element "0, 0, 0" 0.0001)
      (Math|Integer|IncrementInt (LocalVariables|GetIter))))
  (if (== 0 (LocalVariables|GetIter))
    (return true)
    (else
      (return false))))

(fn GeneratePositions
  (params (Genes :type Array%20of%20Strings))
  (bind _returnvalue (Class|ReadInputFile|GenerateGeneVectors (Utilities|Array|Length Genes)))
  (return _returnvalue))

(fn SortGenesAlphabetically
  (bind _outactors (Actor|GetAllActorsOfClass 0 "/Game/Blueprints/Exon_Intron_Model.Exon_Intron_Model_C"))
  (for _array_element _outactors
    (Utilities|Array|Add (LocalVariables|GetUnsortedNames) (Variables|/Game/Blueprints/Exon_Intron_Model.Exon_Intron_Model_C|GetGeneName _array_element)))
  (bind _returnvalue (Class|AutoLayout|SortGenesAlphabetically (LocalVariables|GetUnsortedNames)))
  (bind _output_get (LocalVariables|SetSortedNames _returnvalue))
  (bind _returnvalue_2 (Class|AutoLayout|GetAlphabeticalVectors _output_get))
  (LocalVariables|SetSortedLocations _returnvalue_2)
  (bind _outactors_2 (Actor|GetAllActorsOfClass 0 "/Game/Blueprints/Exon_Intron_Model.Exon_Intron_Model_C"))
  (for _array_element_2 _outactors_2
    (Transformation|SetActorLocationAndRotation _array_element_2 (Utilities|Array|Get(acopy) (LocalVariables|GetSortedLocations) (Utilities|Array|FindItem (LocalVariables|GetSortedNames) (Variables|/Game/Blueprints/Exon_Intron_Model.Exon_Intron_Model_C|GetGeneName _array_element_2))) "0,-90.000000, 0")
    (Default|MoveSpline _array_element_2)))

(fn SortGenesConnectivity
  (bind _unsortedints (LocalVariables|GetUnsortedInts))
  (bind _unsortedints_2 (LocalVariables|GetUnsortedInts))
  (bind _outactors (Actor|GetAllActorsOfClass 0 "/Game/Blueprints/Exon_Intron_Model.Exon_Intron_Model_C"))
  (for _array_element _outactors
    (Utilities|Array|Add (LocalVariables|GetGeneNames) (Variables|/Game/Blueprints/Exon_Intron_Model.Exon_Intron_Model_C|GetGeneName _array_element)))
  (for _array_element_2 (LocalVariables|GetGeneNames)
    (Utilities|Array|Add (LocalVariables|GetUnsortedInts) (Class|KismetSystemLibrary|MakeLiteralInteger)))
  (bind _outactors_2 (Actor|GetAllActorsOfClass 0 "/Game/Blueprints/Network_Model.Network_Model_C"))
  (for _array_element_3 _outactors_2
    (Utilities|Array|SetArrayElem _unsortedints_2 (Utilities|Array|FindItem (LocalVariables|GetGeneNames) (Variables|/Game/Blueprints/Network_Model.Network_Model_C|GetStart%20Gene _array_element_3)) (+ (Utilities|Array|Get(acopy) _unsortedints_2 (Utilities|Array|FindItem (LocalVariables|GetGeneNames) (Variables|/Game/Blueprints/Network_Model.Network_Model_C|GetStart%20Gene _array_element_3))) 1))
    (Utilities|Array|SetArrayElem _unsortedints (Utilities|Array|FindItem (LocalVariables|GetGeneNames) (Variables|/Game/Blueprints/Network_Model.Network_Model_C|GetEnd%20Gene _array_element_3)) (+ (Utilities|Array|Get(acopy) _unsortedints (Utilities|Array|FindItem (LocalVariables|GetGeneNames) (Variables|/Game/Blueprints/Network_Model.Network_Model_C|GetEnd%20Gene _array_element_3))) 1)))
  (bind _returnvalue (Class|AutoLayout|SortUnsortedInts (LocalVariables|GetUnsortedInts)))
  (bind _output_get (LocalVariables|SetSortedInts _returnvalue))
  (bind _returnvalue_2 (Class|AutoLayout|MatchGeneNames (LocalVariables|GetUnsortedInts) _output_get (LocalVariables|GetGeneNames)))
  (LocalVariables|SetMatchedGeneNames _returnvalue_2)
  (bind _returnvalue_3 (Class|AutoLayout|GenerateConnectivityLocations (LocalVariables|GetSortedInts)))
  (LocalVariables|SetLocationVectors _returnvalue_3)
  (bind _outactors_3 (Actor|GetAllActorsOfClass 0 "/Game/Blueprints/Exon_Intron_Model.Exon_Intron_Model_C"))
  (for _array_element_4 _outactors_3
    (Transformation|SetActorLocationAndRotation _array_element_4 (Utilities|Array|Get(acopy) (LocalVariables|GetLocationVectors) (Utilities|Array|FindItem (LocalVariables|GetMatchedGeneNames) (Variables|/Game/Blueprints/Exon_Intron_Model.Exon_Intron_Model_C|GetGeneName _array_element_4))) "0,-90.000000, 0")
    (Default|MoveSpline _array_element_4)))