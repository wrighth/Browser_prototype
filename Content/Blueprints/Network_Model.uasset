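; Network_Model is an actor that draws a spline-mesh link between its StartNode and EndNode actors.
; The construction script builds a two-point spline from their world locations, then feeds local positions and tangents into spline meshes attached to the root.
; The first mesh spans the two points with a custom up direction; a second requests a nonexistent third point.
; The event graph has no runtime logic.
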(event EventBeginPlay)

(event Collision|EventActorBeginOverlap
  (params (OtherActor :type Actor%20Object%20Reference)))

(event EventTick
  (params (DeltaSeconds :type Float%20%28single-precision%29)))

(fn ConstructionScript
  (bind _returnvalue (AddComponent|AddSplineComponent false))
  (Spline|ClearSplinePoints _returnvalue)
  (Spline|AddSplinePoint _returnvalue (Transformation|GetActorLocation (Variables|Default|GetStart%20Node)) "World")
  (Spline|AddSplinePoint _returnvalue (Transformation|GetActorLocation (Variables|Default|GetEnd%20Node)) "World")
  (bind _returnvalue_2 (AddComponent|AddSplineMeshComponent false))
  (Transformation|AttachComponentToComponent _returnvalue_2 (Variables|Default|GetDefaultSceneRoot) "None" "KeepRelative" "KeepRelative" "KeepRelative" true)
  (SplineMesh|SetSplineUpDir _returnvalue_2 (Math|Vector|MakeVector 0.0 -9e+01 0.0) true)
  (SplineMesh|SetStartandEnd _returnvalue_2 (.Location (Spline|GetLocationandTangentatSplinePoint _returnvalue 0 "Local")) (.Tangent (Spline|GetLocationandTangentatSplinePoint _returnvalue 0 "Local")) (.Location (Spline|GetLocationandTangentatSplinePoint _returnvalue 1 "Local")) (.Tangent (Spline|GetLocationandTangentatSplinePoint _returnvalue 1 "Local")) true :!class /Script/Engine.SplineMeshComponent)
  (bind _returnvalue_3 (AddComponent|AddSplineMeshComponent false))
  (Transformation|AttachComponentToComponent _returnvalue_3 (Variables|Default|GetDefaultSceneRoot) "None" "KeepRelative" "KeepRelative" "KeepRelative" true)
  (SplineMesh|SetStartandEnd _returnvalue_3 (.Location (Spline|GetLocationandTangentatSplinePoint _returnvalue 1 "Local")) (.Tangent (Spline|GetLocationandTangentatSplinePoint _returnvalue 1 "Local")) (.Location (Spline|GetLocationandTangentatSplinePoint _returnvalue 2 "Local")) (.Tangent (Spline|GetLocationandTangentatSplinePoint _returnvalue 2 "Local")) true :!class /Script/Engine.SplineMeshComponent))